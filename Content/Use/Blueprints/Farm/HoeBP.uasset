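; HoeBP is a hoe pickup actor that the player collects with the Interact input.
; Its Ww overlap component caches the C_Player, enables input and opens a gate on entry, then disables input and closes the gate on exit.
; Interact through the open gate sets the player's HasHoe flag and destroys the actor, while a player who already has a hoe only triggers a debug print.
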(event OnComponentBeginOverlap(ww)
  (params (OverlappedComponent :type Primitive%20Component%20Object%20Reference) (OtherActor :type Actor%20Object%20Reference) (OtherComp :type Primitive%20Component%20Object%20Reference) (OtherBodyIndex :type Integer) (bFromSweep :type Boolean) (SweepResult :type Hit%20Result%20Structure%20%28by%20ref%29))
  (bind _asc_player (Utilities|Casting|CastToC_Player OtherActor))
  (Input|EnableInput (Game|GetPlayerController 0))
  (Utilities|FlowControl|Gate true) ; enters at Open
)

(event OnComponentEndOverlap(ww)
  (params (OverlappedComponent :type Primitive%20Component%20Object%20Reference) (OtherActor :type Actor%20Object%20Reference) (OtherComp :type Primitive%20Component%20Object%20Reference) (OtherBodyIndex :type Integer))
  (Utilities|Casting|CastToC_Player OtherActor)
  (Input|DisableInput (Game|GetPlayerController 0))
  (Utilities|FlowControl|Gate true) ; enters at Close
)

(event Input|ActionEvents|InputActionInteract
  (params (Key :type Key%20Structure :default "None"))
  (:Pressed
    (if (Variables|/Game/Use/Character/C_Player.C_Player_C|GetHasHoe? (stale OnComponentBeginOverlap(ww) _asc_player))
      (Development|PrintString "Go Farm")
      (else
        (Utilities|FlowControl|Gate true
          (:Exit
            (Variables|/Game/Use/Character/C_Player.C_Player_C|SetHasHoe? (stale OnComponentBeginOverlap(ww) _asc_player) true)
            (Actor|DestroyActor)
            (Development|PrintString "Pick Hoe")))))))

(fn ConstructionScript)