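; LastDoor is a door actor that opens only for a player holding the last key.
; When a C_Player overlaps the R component and HasLastKey is true, the DoorPlay timeline plays and offsets the Plate's relative Z by its DoorTrack value times Move.
; The timeline reverses whenever a C_Player leaves the overlap, without checking the key.
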(event OnComponentBeginOverlap(r)
  (params (OverlappedComponent :type Primitive%20Component%20Object%20Reference) (OtherActor :type Actor%20Object%20Reference) (OtherComp :type Primitive%20Component%20Object%20Reference) (OtherBodyIndex :type Integer) (bFromSweep :type Boolean) (SweepResult :type Hit%20Result%20Structure%20%28by%20ref%29))
  (bind _asc_player (Utilities|Casting|CastToC_Player OtherActor))
  (if (Variables|/Game/Use/Character/C_Player.C_Player_C|GetHasLastKey? _asc_player)
    (bind _doortrack (Timeline|DoorPlay Play)
      (:Update
        (Transformation|SetRelativeLocation (Variables|Default|GetPlate) (Math|Vector|MakeVector 0.0 0.0 (* _doortrack (Variables|Default|GetMove))) false false)))))

(event OnComponentEndOverlap(r)
  (params (OverlappedComponent :type Primitive%20Component%20Object%20Reference) (OtherActor :type Actor%20Object%20Reference) (OtherComp :type Primitive%20Component%20Object%20Reference) (OtherBodyIndex :type Integer))
  (Utilities|Casting|CastToC_Player OtherActor)
  (bind _doortrack (Timeline|DoorPlay Reverse)
    (:Update
      (Transformation|SetRelativeLocation (Variables|Default|GetPlate) (Math|Vector|MakeVector 0.0 0.0 (* _doortrack (Variables|Default|GetMove))) false false))))

(event EventBeginPlay)

(event Collision|EventActorBeginOverlap
  (params (OtherActor :type Actor%20Object%20Reference)))

(event EventTick
  (params (DeltaSeconds :type Float%20%28single-precision%29)))

(fn ConstructionScript)